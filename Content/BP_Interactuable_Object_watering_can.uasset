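; Watering can interactable that refills a plant's water level, with a limited number of uses.
; Overlapping a BP_Plant stores it as the target, and overlapping a BP_Tub refills the can only once it is empty.
; Effect resets the stored plant's water and spends a use even without a valid plant, printing status messages.
; Respawn spawns a fresh can at the initial position and destroys this one.
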(event EventBeginPlay
  (|CallParentFunction)
  ;[0.15 0.15 0.15 0.5 14] Setteo de variables
  (Variables|Default|Setuses (Variables|Default|GetmaxUses))
  (Variables|Default|SetstaticMesh (Variables|Default|GetCylinder))
  (Variables|Default|SetinitPos (Transformation|GetActorLocation))
  (Variables|Default|Setcollider (Variables|Default|GetBoxCollider)))

(event Collision|EventActorBeginOverlap
  (params (OtherActor :type Actor%20Object%20Reference))
  (|CallParentFunction OtherActor)
  ;[0.15 0.15 0.15 0.5] Guardar la planta
  (bind _asbp_plant (Utilities|Casting|CastToBP_Plant OtherActor)
    (:then
      (Variables|Default|Setplant _asbp_plant))
    (:CastFailed
      ;[0.15 0.15 0.15 0.5] Rellenar la regadera
      (Utilities|Casting|CastToBP_Tub OtherActor)
      (if (<= (Variables|Default|Getuses) 0)
        (Variables|Default|Setuses (Variables|Default|GetmaxUses))
        (Development|PrintString "Regadera llena")))))

(event EventTick
  (params (DeltaSeconds :type Float%20%28single-precision%29))
  (|CallParentFunction DeltaSeconds))

(fn ConstructionScript
  (|CallParentFunction))

(fn Effect
  (bind _plant (Variables|Default|Getplant))
  (|CallParentFunction)
  ;[0.15 0.15 0.15 0.5] Si no esta vacia
  (if (> (Variables|Default|Getuses) 0)
    ;[0.15 0.15 0.15 0.5] Relleno el nivel de agua de la planta
    (Utilities|IsValid _plant
      (:Is%20Valid
        (Default|ResetWaterLevel _plant))
      (:Is%20Not%20Valid
        _))
    ;[0.15 0.15 0.15 0.5] Resto 1 uso
    (if (<= (- (Variables|Default|Getuses) 1) 0)
      ;[0.15 0.15 0.15 0.5] Se queda sin usos
      (Variables|Default|Setuses 0)
      (Development|PrintString "Rellena la regadera")
      (else
        (Variables|Default|Setuses (- (Variables|Default|Getuses) 1))
        (Development|PrintString (Utilities|String|Append "Uses: " (Utilities|String|ToString(Integer) (Variables|Default|Getuses))))))))

(fn Respawn
  (|CallParentFunction)
  (Game|SpawnActorfromClass "BP_Interactuable_Object_watering_can_C" (Math|Transform|MakeTransform (Variables|Default|GetinitPos) "0, 0, 0" "1.000000,1.000000,1.000000") "Undefined" "MultiplyWithRoot" 0 0)
  (Actor|DestroyActor))