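; BP_Plant is a plant actor that tracks a water level which drains over time.
; On BeginPlay a looping timer calls WaterUpdate, which subtracts a decrement and clamps the level at zero.
; Tick checks the level every frame and refills it to the starting value once empty, a behavior an in-file note marks to be changed.
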(event Custom|WaterEvent
  ;[0.15 0.15 0.15 0.5] Evento que resta agua
  (CallFunction|WaterUpdate))

(event EventBeginPlay
  ;[0.15 0.15 0.15 0.5] Evento que resta agua
  (Utilities|Time|SetTimerbyEvent (delegate Custom|WaterEvent) (Variables|Default|Gettime) true))

(event Collision|EventActorBeginOverlap
  (params (OtherActor :type Actor%20Object%20Reference)))

(event EventTick
  (params (DeltaSeconds :type Float%20%28single-precision%29))
  ;[0.15 0.15 0.15 0.5] Si se queda sin agua se rellena, cambiar
  (if (<= (Variables|Default|GetcurrentWaterLevel) 0.0)
    (CallFunction|ResetWaterLevel)
    (else
      (Development|PrintString ""))))

(fn ConstructionScript)

(fn WaterUpdate
  (if (<= (- (Variables|Default|GetcurrentWaterLevel) (Variables|Default|GetwaterDecrement)) 0.0)
    (Variables|Default|SetcurrentWaterLevel 0.0)
    (else
      (Variables|Default|SetcurrentWaterLevel (- (Variables|Default|GetcurrentWaterLevel) (Variables|Default|GetwaterDecrement))))))

(fn ResetWaterLevel
  (Variables|Default|SetcurrentWaterLevel (Variables|Default|GetwaterLevel)))