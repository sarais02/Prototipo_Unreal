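; Interactable pickup object that a third-person character carries on its head and that can be used to trigger an effect.
; On overlap it stores the player, attaches to the capsule and moves above it using capsule and cylinder heights.
; Tick runs Effect when grabbed and Activated, a flag this Blueprint never sets true.
; Effect is a placeholder print that immediately despawns the object, zeroing BP_Spawner's counter.
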(event EventBeginPlay
  ;[0.15 0.15 0.15 0.5 14] Setteo los bools a false
  (Variables|Default|Setgrabbed false)
  (Variables|Default|Setactivated false)
  ;[0.15 0.15 0.15 0.5 14] Referencia al spawner
  (bind _returnvalue (Actor|GetActorOfClass "/Game/BP_Spawner.BP_Spawner_C"))
  (Variables|Default|Setspawner _returnvalue))

(event Collision|EventActorBeginOverlap
  (params (OtherActor :type Actor%20Object%20Reference))
  ;[0.15 0.15 0.15 0.5 14] Guardo la info del player
  (bind _asbp_third_person_character (Utilities|Casting|CastToBP_ThirdPersonCharacter OtherActor))
  (Variables|Default|Setplayer _asbp_third_person_character)
  ;[0.15 0.15 0.15 0.5 14] Lo marco como cogido
  (Variables|Default|Setgrabbed true)
  ;[0.15 0.15 0.15 0.5] Colocar el objeto en la cabeza del jugador
  (Transformation|AttachComponentToComponent (Variables|/Script/Engine.Character|GetCapsuleComponent _asbp_third_person_character) "None" "SnapToTarget" "SnapToTarget" "KeepRelative" true)
  (Transformation|SetActorLocation (+ (Transformation|GetActorLocation (Variables|Default|Getplayer)) (Math|Vector|MakeVector 0.0 0.0 (+ (Components|Capsule|GetUnscaledCapsuleHalfHeight (Variables|/Script/Engine.Character|GetCapsuleComponent _asbp_third_person_character)) (/ (.z (.Max (Components|StaticMesh|GetLocalBounds (Variables|Default|GetCylinder)))) 2.0)))) false false))

(event EventTick
  (params (DeltaSeconds :type Float%20%28single-precision%29))
  ;[0.15 0.15 0.15 0.5 14] Si lo ha cogido y lo usa, se activa su efecto
  (if (and (Variables|Default|Getgrabbed) (Variables|Default|Getactivated))
    (CallFunction|Effect)))

(fn ConstructionScript)

(fn Effect
  ;[0.15 0.15 0.15 0.5 14] Al usarlo, se destruye a los 2 segundos
  (Development|PrintString "Efecto")
  (if (Variables|Default|Getgrabbed)
    (CallFunction|Despawn)))

(fn Despawn
  ;[0.15 0.15 0.15 0.5 14] Se elimina el objeto, en la escena y en el spawner
  (Variables|/Game/BP_Spawner.BP_Spawner_C|Setcont (Variables|Default|Getspawner) 0)
  (Actor|DestroyActor))