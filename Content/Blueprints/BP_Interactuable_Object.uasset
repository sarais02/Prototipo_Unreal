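; BP_Interactuable_Object is an interactable pickup that the third-person character carries on its head.
; On overlap it stores the player, disables its collider, attaches to the capsule and sits above it using capsule height and mesh bounds.
; Detach releases it and enables mesh physics; Respawn moves the root to InitPos, which is not set here.
; Effect is a stub that prints and, while grabbed, clears Activated.
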(event EventBeginPlay
  ;[0.15 0.15 0.15 0.5 14] Setteo los bools a false
  (Variables|Default|Setgrabbed false)
  (Variables|Default|Setactivated false))

(event Collision|EventActorBeginOverlap
  (params (OtherActor :type Actor%20Object%20Reference))
  ;[0.15 0.15 0.15 0.5 14] Guardo la info del player
  (bind _asbp_third_person_character (Utilities|Casting|CastToBP_ThirdPersonCharacter OtherActor))
  (Variables|Default|Setplayer _asbp_third_person_character)
  ;[0.15 0.15 0.15 0.5 14] Lo marco como cogido
  (Variables|Default|Setgrabbed true)
  ;[0.15 0.15 0.15 0.5] Colocar el objeto en la cabeza del jugador
  (Collision|SetCollisionEnabled (Variables|Default|Getcollider) "NoCollision")
  (Transformation|AttachComponentToComponent (Variables|/Script/Engine.Character|GetCapsuleComponent _asbp_third_person_character) "None" "SnapToTarget" "SnapToTarget" "KeepWorld" true)
  (Transformation|SetActorLocation (+ (Transformation|GetActorLocation (Variables|Default|Getplayer)) (Math|Vector|MakeVector 0.0 0.0 (+ (Components|Capsule|GetUnscaledCapsuleHalfHeight (Variables|/Script/Engine.Character|GetCapsuleComponent _asbp_third_person_character)) (/ (.z (.BoxExtent (Collision|GetComponentBounds (Variables|Default|GetstaticMesh)))) 2.0)))) false false)
  (Transformation|SetActorRotation "0, 0, 0"))

(fn ConstructionScript)

(fn Effect
  ;[0.15 0.15 0.15 0.5 14] Al usarlo
  (Development|PrintString "Efecto")
  (if (Variables|Default|Getgrabbed)
    (Variables|Default|Setactivated false)))

(fn Detach
  ;[0.15 0.15 0.15 0.5] Soltar objeto
  (Variables|Default|Setgrabbed false)
  (Development|PrintString "DETACH" true true "(R=0.058024,G=1.000000,B=0.000000,A=1.000000)")
  (Transformation|DetachFromActor "KeepRelative" "KeepRelative" "KeepRelative")
  (Transformation|AttachComponentToComponent (Variables|Default|Getcollider) (Variables|Default|GetstaticMesh) "None" "SnapToTarget" "SnapToTarget" "KeepWorld" true)
  (Physics|SetSimulatePhysics (Variables|Default|GetstaticMesh) true))

(fn Respawn
  (Transformation|SetWorldLocation (Variables|Default|GetDefaultSceneRoot) (Variables|Default|GetinitPos) false false)
  (Development|PrintString "RESPAWN" true true "(R=0.364264,G=1.000000,B=0.000000,A=1.000000)" 5.0))