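; Watering can, a child interactable that waters plants and tracks its remaining uses in BP_ThirdPersonGameMode.
; Overlap stores the last plant touched, or refills an empty can at a BP_Tub.
; Effect plays splash particles and sound while uses remain, resets the stored plant's water unless full, and spends a use, even without a plant.
; Respawn spawns a fresh can at the initial location and destroys itself.
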(event EventBeginPlay
  (|CallParentFunction)
  ;[0.15 0.15 0.15 0.5 14] Setteo de variables
  (bind _asbp_third_person_game_mode (Utilities|Casting|CastToBP_ThirdPersonGameMode (Game|GetGameMode)))
  (Variables|Default|SetgameMode _asbp_third_person_game_mode)
  (Variables|Default|SetstaticMesh (Variables|Default|GetCylinder))
  (Variables|Default|SetinitPos (Transformation|GetActorLocation))
  (Variables|Default|Setcollider (Variables|Default|GetBoxCollider))
  (bind _asbp_water_splash (Utilities|Casting|CastToBP_WaterSplash (Variables|/Script/Engine.ChildActorComponent|GetChildActor (Variables|Default|GetParticles))))
  (Variables|Default|SetwaterParticles _asbp_water_splash))

(event Collision|EventActorBeginOverlap
  (params (OtherActor :type Actor%20Object%20Reference))
  (bind _gamemode (Variables|Default|GetgameMode))
  (|CallParentFunction OtherActor)
  ;[0.15 0.15 0.15 0.5] Guardar la planta
  (bind _asbp_plant (Utilities|Casting|CastToBP_Plant OtherActor)
    (:then
      (Variables|Default|Setplant _asbp_plant))
    (:CastFailed
      ;[0.15 0.15 0.15 0.5] Rellenar la regadera
      (Utilities|Casting|CastToBP_Tub OtherActor)
      (if (<= (Variables|/Game/ThirdPerson/Blueprints/BP_ThirdPersonGameMode.BP_ThirdPersonGameMode_C|GetwaterUses (Variables|Default|GetgameMode)) 0)
        (Variables|/Game/ThirdPerson/Blueprints/BP_ThirdPersonGameMode.BP_ThirdPersonGameMode_C|SetwaterUses _gamemode (Variables|/Game/ThirdPerson/Blueprints/BP_ThirdPersonGameMode.BP_ThirdPersonGameMode_C|GetmaxWaterUses _gamemode))
        (Audio|PlaySound2D "/Game/Musica_Sonidos/fill-water-192164.fill-water-192164" 0.5 1.0 0.0 0 0)
        (Default|Start (Variables|Default|GetwaterParticles))
        (Development|PrintString "Regadera llena")))))

(event EventTick
  (params (DeltaSeconds :type Float%20%28single-precision%29))
  (|CallParentFunction DeltaSeconds))

(fn ConstructionScript
  (|CallParentFunction))

(fn Effect
  (bind _plant (Variables|Default|Getplant))
  (|CallParentFunction)
  ;[0.15 0.15 0.15 0.5] Si no esta vacia
  (if (> (Variables|/Game/ThirdPerson/Blueprints/BP_ThirdPersonGameMode.BP_ThirdPersonGameMode_C|GetwaterUses (Variables|Default|GetgameMode)) 0)
    (Default|Start (Variables|Default|GetwaterParticles))
    ;[0.15 0.15 0.15 0.5] Relleno el nivel de agua de la planta si lo necesita
    (Audio|PlaySound2D "/Game/Musica_Sonidos/fill-water-192164.fill-water-192164" 0.5 1.0 0.0 0 0)
    (Utilities|IsValid _plant
      (:Is%20Valid
        (bind _isfull (Default|IsFull _plant))
        (if (not _isfull)
          (Default|ResetWaterLevel _plant)
          ;[0.15 0.15 0.15 0.5] Resto 1 uso
          (if (<= (- (Variables|/Game/ThirdPerson/Blueprints/BP_ThirdPersonGameMode.BP_ThirdPersonGameMode_C|GetwaterUses (Variables|Default|GetgameMode)) 1) 0) :!label _label
            ;[0.15 0.15 0.15 0.5] Se queda sin usos
            (Variables|/Game/ThirdPerson/Blueprints/BP_ThirdPersonGameMode.BP_ThirdPersonGameMode_C|SetwaterUses (Variables|Default|GetgameMode) 0)
            (Development|PrintString "Rellena la regadera")
            (else
              (Variables|/Game/ThirdPerson/Blueprints/BP_ThirdPersonGameMode.BP_ThirdPersonGameMode_C|SetwaterUses (Variables|Default|GetgameMode) (- (Variables|/Game/ThirdPerson/Blueprints/BP_ThirdPersonGameMode.BP_ThirdPersonGameMode_C|GetwaterUses (Variables|Default|GetgameMode)) 1))
              (Development|PrintString (Utilities|String|Append "Uses: " (Utilities|String|ToString(Integer) (Variables|/Game/ThirdPerson/Blueprints/BP_ThirdPersonGameMode.BP_ThirdPersonGameMode_C|GetwaterUses (Variables|Default|GetgameMode)))))))))
      (:Is%20Not%20Valid
        (goto _label)))))

(fn Respawn
  (|CallParentFunction)
  (Game|SpawnActorfromClass "BP_Interactuable_Object_watering_can_C" (Math|Transform|MakeTransform (Variables|Default|GetinitPos) "0, 0, 0" "1.000000,1.000000,1.000000") "Undefined" "MultiplyWithRoot" 0 0)
  (Actor|DestroyActor))