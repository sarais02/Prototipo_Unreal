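; BP_Interactuable_Object_Spray is an interactable spray object that replenishes a plant's timer, built on a parent class with Effect, Detach and Respawn hooks.
; Overlapping a BP_Plant stores it and resets its time to the maximum; Effect sets it to maximum plus a bonus, then despawns the spray.
; Despawning, also triggered by Respawn, zeroes the BP_Spawner counter and destroys the actor.
; A repeating-reset timer node is left unconnected.
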(event Custom|ResetTimerPlant
  (CallFunction|ResetTimer))

(event EventBeginPlay
  (|CallParentFunction)
  ;[0.15 0.15 0.15 0.5 14] Referencia al spawner
  (bind _returnvalue (Actor|GetActorOfClass "/Game/Blueprints/BP_Spawner.BP_Spawner_C"))
  (Variables|Default|SetSpawner _returnvalue)
  ;[0.15 0.15 0.15 0.5 14] Setteo de variables
  (Variables|Default|SetstaticMesh (Variables|Default|GetCylinder))
  (Variables|Default|SetinitPos (Transformation|GetActorLocation))
  (Variables|Default|Setcollider (Variables|Default|GetBoxCollider)))

(event Collision|EventActorBeginOverlap
  (params (OtherActor :type Actor%20Object%20Reference))
  (|CallParentFunction OtherActor)
  (bind _asbp_plant (Utilities|Casting|CastToBP_Plant OtherActor))
  (Variables|Default|Setplant _asbp_plant)
  (CallFunction|ResetTimer))

(event EventTick
  (params (DeltaSeconds :type Float%20%28single-precision%29))
  (|CallParentFunction DeltaSeconds))

(fn ConstructionScript
  (|CallParentFunction))

(fn Despawn
  (Variables|/Game/Blueprints/BP_Spawner.BP_Spawner_C|Setcont (Variables|Default|GetSpawner) 0)
  (Actor|DestroyActor))

(fn Effect
  (bind _plant (Variables|Default|Getplant))
  (|CallParentFunction)
  (Variables|/Game/Blueprints/BP_Plant.BP_Plant_C|Settime _plant (+ (Variables|/Game/Blueprints/BP_Plant.BP_Plant_C|GetmaxTime _plant) (Variables|Default|GettimeIncrement)))
  (CallFunction|Despawn))

(fn ResetTimer
  (bind _plant (Variables|Default|Getplant))
  (Variables|/Game/Blueprints/BP_Plant.BP_Plant_C|Settime _plant (Variables|/Game/Blueprints/BP_Plant.BP_Plant_C|GetmaxTime _plant)))

(fn Detach
  (|CallParentFunction))

(fn Respawn
  (|CallParentFunction)
  (CallFunction|Despawn))